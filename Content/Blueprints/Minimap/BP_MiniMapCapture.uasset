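; BP_MiniMapCapture is a helper actor that captures a map view and saves it as a minimap PNG.
; Its construction script sets the scene capture's ortho width, render target and hidden actor list.
; On BeginPlay it adds PlayerInterface actors to that hidden list, exports T_MiniMapRenderTarget under the project directory using the minimap name, then destroys itself.
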(event Custom|ExportMapImage
  ;[1 1 1] Export image
  (Rendering|ExportRenderTarget "/Game/TopDownRPGTemplate/Textures/T_MiniMapRenderTarget.T_MiniMapRenderTarget" (Utilities|String|Append (Class|KismetSystemLibrary|GetProjectDirectory) (Variables|Default|Getpath)) (Utilities|String|Append "T_" (Variables|Default|GetminiMapName) ".png")))

(event Custom|HideAllInteractrables
  (bind _ignoreactors (Variables|Default|GetignoreActors))
  ;[1 1 1] Hide interactables
  (bind _outactors (Actor|GetAllActorswithInterface "/Script/PJ_AURA.PlayerInterface"))
  (Utilities|Array|AppendArray _ignoreactors _outactors)
  (Variables|/Script/Engine.SceneCaptureComponent|SetHiddenActors (Variables|Default|GetSceneCaptureComponent2D) _ignoreactors))

(event EventBeginPlay
  ;[1 1 1] Destroy at begin play
  (CallFunction|HideAllInteractrables)
  (CallFunction|ExportMapImage)
  (Actor|DestroyActor))

(fn ConstructionScript
  ;[1 1 1] Set minimap details
  (Variables|/Script/Engine.SceneCaptureComponent2D|SetOrthoWidth (Variables|Default|GetSceneCaptureComponent2D) (Variables|Default|GetmapSize))
  (Variables|/Script/Engine.SceneCaptureComponent2D|SetTextureTarget (Variables|Default|GetSceneCaptureComponent2D) (Variables|Default|GetminiMapRenderTarget))
  (Variables|/Script/Engine.SceneCaptureComponent|SetHiddenActors (Variables|Default|GetSceneCaptureComponent2D) (Variables|Default|GetignoreActors)))