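; Minimap detector that uses a sphere to decide which nearby actors show icons on the minimap.
; Begin overlap routes through OnDetectorOverlap, which calls ShowMiniMapIcon for actors implementing MiniMapInterface, excluding AuraActor.
; End overlap calls RemoveMiniMapIcon on any departing actor without the same filter.
; Both paths print debug text, and InitializeMinimapDetector is an empty stub.
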(event OnComponentBeginOverlap(Sphere)
  (params (OverlappedComponent :type Primitive%20Component%20Object%20Reference) (OtherActor :type Actor%20Object%20Reference) (OtherComp :type Primitive%20Component%20Object%20Reference) (OtherBodyIndex :type Integer) (bFromSweep :type Boolean) (SweepResult :type Hit%20Result%20Structure%20%28by%20ref%29))
  (CallFunction|OnDetectorOverlap OtherActor))

(event OnComponentEndOverlap(Sphere)
  (params (OverlappedComponent :type Primitive%20Component%20Object%20Reference) (OtherActor :type Actor%20Object%20Reference) (OtherComp :type Primitive%20Component%20Object%20Reference) (OtherBodyIndex :type Integer))
  (CallFunction|RemoveMiniMapIcon OtherActor)
  (Development|PrintText (Utilities|Text|FormatText (Utilities|Text|MakeLiteralText "EndOverlapping{0}") (Utilities|GetObjectName OtherActor))))

(event Custom|InitializeMinimapDetector)

(event Custom|OnDetectorOverlap
  (params (actor :type Actor%20Object%20Reference))
  (if (Utilities|DoesObjectImplementInterface actor "/Script/PJ_AURA.MiniMapInterface")
    (if (not (== (Variables|Default|GetAuraActor) actor))
      (CallFunction|ShowMiniMapIcon actor)
      (Development|PrintText (Utilities|Text|FormatText (Utilities|Text|MakeLiteralText "Overlapping{0}") (Utilities|GetObjectName actor))))))

(event EventBeginPlay)

(event Collision|EventActorBeginOverlap
  (params (OtherActor :type Actor%20Object%20Reference)))

(event EventTick
  (params (DeltaSeconds :type Float%20%28single-precision%29)))

(fn ConstructionScript)