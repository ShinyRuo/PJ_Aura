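; Blueprint function library with helpers that add or remove an actor's icon on the player's minimap.
; Both functions reach the minimap widget by casting player 0's HUD to AuraHUD and its overlay widget to WBP_Overlay, silently stopping if either cast fails.
; Showing queries the actor itself for icon, permanence, rotation and removal settings and forwards them to the minimap, while removal passes only the actor.
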(fn ShowMiniMapIcon
  (params (actor :type Actor%20Object%20Reference))
  ;[1 1 1] Show minimap icon
  (bind _asaura_hud (Utilities|Casting|CastToAuraHUD (HUD|GetHUD (Game|GetPlayerController 0))))
  (bind _aswbp_overlay (Utilities|Casting|CastToWBP_Overlay (Class|AuraHUD|GetOverlayWidget _asaura_hud)))
  (bind (_outminimapicon _outispermanent _outshouldremoveicon _outignoremaprotation) (Class|MiniMapInterface|GetMiniMapIcon(Message) actor))
  (Default|ShowMiniMapIcon (Variables|/Game/Blueprints/UI/Overlay/WBP_Overlay.WBP_Overlay_C|GetWBP_Minimap _aswbp_overlay) actor _outminimapicon _outispermanent _outignoremaprotation _outshouldremoveicon))

(fn RemoveMiniMapIcon
  (params (actor :type Actor%20Object%20Reference))
  (bind _asaura_hud (Utilities|Casting|CastToAuraHUD (HUD|GetHUD (Game|GetPlayerController 0))))
  (bind _aswbp_overlay (Utilities|Casting|CastToWBP_Overlay (Class|AuraHUD|GetOverlayWidget _asaura_hud)))
  (Default|RemoveMiniMapIcon (Variables|/Game/Blueprints/UI/Overlay/WBP_Overlay.WBP_Overlay_C|GetWBP_Minimap _aswbp_overlay) actor))