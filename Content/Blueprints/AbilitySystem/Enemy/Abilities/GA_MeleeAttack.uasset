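; Enemy melee attack gameplay ability that faces the combat target and plays a random attack montage.
; The montage's gameplay event triggers a sphere check at its tagged combat socket, damaging live non-friendly players.
; A hit fires the MeleeImpact gameplay cue tagged with the montage tag.
; A miss ends the ability immediately without stopping the montage; otherwise it ends when the montage finishes or is interrupted.
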(event Ability|EventActivateAbility
  (Variables|Default|SetHasHitTarget false)
  (Variables|Default|SetOwningActor (Ability|GetAvatarActorfromActorInfo))
  (bind _returnvalue (Class|EnemyInterface|GetCombatTarget(Message) (Variables|Default|GetOwningActor)))
  (bind _ascombat_interface (Utilities|Casting|CastToCombatInterface (Variables|Default|GetOwningActor)))
  (Class|CombatInterface|UpdateFacingTarget _ascombat_interface (Transformation|GetActorLocation _returnvalue))
  (bind _returnvalue_2 (Class|CombatInterface|GetAttackMontages(Message) (Variables|Default|GetOwningActor)))
  (bind _output_get (Variables|Default|SetThisTimeMontageInfo (.OutItem (Utilities|Array|Random _returnvalue_2))))
  (Variables|Default|SetThisTimeTag_Montage (.MontageTag (Utilities|Struct|BreakTaggedMontage _output_get)))
  (Variables|Default|SetThisTimeTag_Socket (.SocketTag (Utilities|Struct|BreakTaggedMontage _output_get)))
  (|PlayMontageandWaitProxy "None" (.Montage (Utilities|Struct|BreakTaggedMontage _output_get)) 1.0 "None" false 1.0 0.0
    (:then
      (Ability|Tasks|WaitGameplayEvent (Variables|Default|GetThisTimeTag_Montage) 0 true
        (:EventReceived
          (bind _ascombat_interface_2 (Utilities|Casting|CastToCombatInterface (Variables|Default|GetOwningActor)))
          (bind _returnvalue_3 (Class|AuraCharacterBase|GetCombatSocketLocation _ascombat_interface_2 (Variables|Default|GetThisTimeTag_Socket)))
          (Variables|Default|SetHitLocation _returnvalue_3)
          (bind _outoverlappingactors (Class|AuraAbilitySystemLibrary|GetLivePlayersWithinRadius (Variables|Default|GetOwningActor) (Utilities|Array|MakeArray (Variables|Default|GetOwningActor)) 45.0 (Variables|Default|GetHitLocation)))
          (for _array_element _outoverlappingactors
            (bind _returnvalue_4 (Class|AuraAbilitySystemLibrary|IsFriend (Variables|Default|GetOwningActor) _array_element))
            (if (not _returnvalue_4)
              (Class|AuraDamageGameplayAbility|CauseDamage _array_element)
              (Variables|Default|SetHasHitTarget true)
              (Class|CombatInterface|GetHitEffect(Message) _array_element)))
          (if (Variables|Default|GetHasHitTarget)
            (bind _returnvalue_5 (Class|EnemyInterface|GetCombatTarget(Message) (Variables|Default|GetOwningActor)))
            (Class|GameplayAbility|ExecuteGameplayCuewithParams "(TagName=\"GameplayCue.MeleeImpact\")" (Ability|GameplayCue|MakeGameplayCueParameters :AggregatedSourceTags (GameplayTags|MakeGameplayTagContainerfromTag (Variables|Default|GetThisTimeTag_Montage)) :Location (Variables|Default|GetHitLocation) :EffectCauser (Variables|Default|GetOwningActor) :SourceObject _returnvalue_5))
            (else
              (Ability|EndAbility))))))
    (:OnCompleted
      (Ability|EndAbility :!label _label))
    (:OnInterrupted
      (goto _label))
    (:OnCancelled
      (goto _label))))

(event Ability|EventOnEndAbility
  (params (bWasCancelled :type Boolean)))