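; Enemy ranged attack ability that turns the avatar toward its combat target and fires a projectile at the target's location captured on activation.
; It plays a random attack montage and waits for a gameplay event with a montage tag, drawn by a separate random evaluation, to spawn the projectile.
; The ability ends shortly after the spawn, or when the montage completes, is interrupted or is cancelled.
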(event Ability|EventActivateAbility
  (Variables|Default|SetOwningActor (Ability|GetAvatarActorfromActorInfo))
  (bind _returnvalue (Class|EnemyInterface|GetCombatTarget(Message) (Variables|Default|GetOwningActor)))
  (bind _ascombat_interface (Utilities|Casting|CastToCombatInterface (Variables|Default|GetOwningActor)))
  (Variables|Default|SetAs%20Combat%20Interface _ascombat_interface)
  (Variables|Default|SetProjectileTargetLocation (Transformation|GetActorLocation _returnvalue))
  (Class|CombatInterface|UpdateFacingTarget _ascombat_interface (Transformation|GetActorLocation _returnvalue))
  (bind _returnvalue_2 (Class|CombatInterface|GetAttackMontages(Message) (Variables|Default|GetOwningActor)))
  (Variables|Default|SetThisTimeTag (.MontageTag (Utilities|Struct|BreakTaggedMontage (.OutItem (Utilities|Array|Random _returnvalue_2)))))
  (|PlayMontageandWaitProxy "None" (.Montage (Utilities|Struct|BreakTaggedMontage (.OutItem (Utilities|Array|Random _returnvalue_2)))) 1.0 "None" false 1.0 0.0
    (:then
      (Ability|Tasks|WaitGameplayEvent (Variables|Default|GetThisTimeTag) 0 true
        (:EventReceived
          (Class|AuraProjectileSpell|SpawnProjectile (Variables|Default|GetProjectileTargetLocation))
          (Utilities|FlowControl|Delay 0.5)
          (Ability|EndAbility))))
    (:OnCompleted
      (Ability|EndAbility :!label _label))
    (:OnInterrupted
      (goto _label))
    (:OnCancelled
      (goto _label))))

(event Ability|EventOnEndAbility
  (params (bWasCancelled :type Boolean)))