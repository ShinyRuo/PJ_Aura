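; Enemy gameplay ability that plays the Shaman summon montage while facing the combat target and spawns random minions.
; Spawn points are derived from the direction to the target, shuffled, and marked with Niagara ground effects while it waits for the montage's attack event.
; That event starts a Delay-based loop spawning staggered, AI-possessed minions facing the target.
; The owner's minion count rises per spawn and falls when each is destroyed.
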(event Custom|OnDestroyed_Event
  (params (DestroyedActor :type Actor%20Object%20Reference))
  (Class|CombatInterface|IncrementMinionCount(Message) (Variables|Default|GetOwningActor) -1))

(event Ability|EventActivateAbility
  (Variables|Default|SetSpawnLocationIndex 0)
  (bind _output_get (Variables|Default|SetOwningActor (Ability|GetAvatarActorfromActorInfo)))
  (bind _returnvalue (Class|EnemyInterface|GetCombatTarget(Message) _output_get))
  (Variables|Default|SetTargetActor _returnvalue)
  (Class|CombatInterface|UpdateFacingTarget(Message) (Variables|Default|GetOwningActor) (Transformation|GetActorLocation (Variables|Default|GetTargetActor)))
  (|PlayMontageandWaitProxy "None" "/Game/Assets/Enemies/Shaman/Animations/AM_Shaman_Summon.AM_Shaman_Summon" 1.0 "None" true 1.0 0.0
    (:then
      (Ability|Tasks|WaitGameplayEvent "(TagName=\"Montage.Attack.1\")" 0 true
        (:then
          (bind _returnvalue_2 (Class|AuraSummonAbility|GetSpawnLocations (Math|Vector|Normalize (- (Transformation|GetActorLocation (Variables|Default|GetTargetActor)) (Transformation|GetActorLocation (Variables|Default|GetOwningActor))))))
          (bind _output_get_2 (Variables|Default|SetSpawnLocations _returnvalue_2))
          (Utilities|Array|Shuffle _output_get_2)
          (for _array_element _output_get_2
            (Niagara|SpawnSystematLocation "/Game/Assets/Effects/Combat/NS_GroundSummon.NS_GroundSummon" _array_element)))
        (:EventReceived
          (if (< (Variables|Default|GetSpawnLocationIndex) (Utilities|Array|Length (Variables|Default|GetSpawnLocations))) :!label _label
            (bind _returnvalue_3 (Game|SpawnActorfromClass (Class|AuraSummonAbility|GetRandomMinionsClass) (Math|Transform|MakeTransform (+ (Utilities|Array|Get(acopy) (Variables|Default|GetSpawnLocations) (Variables|Default|GetSpawnLocationIndex)) "0.000000,0.000000,70.000000") (Math|Rotator|FindLookatRotation (+ (Utilities|Array|Get(acopy) (Variables|Default|GetSpawnLocations) (Variables|Default|GetSpawnLocationIndex)) "0.000000,0.000000,70.000000") (Transformation|GetActorLocation (Variables|Default|GetTargetActor))) "1.000000,1.000000,1.000000") "AlwaysSpawn" "MultiplyWithRoot" 0 0))
            (Game|AssignOnDestroyed _returnvalue_3 (delegate Custom|OnDestroyed_Event))
            (Pawn|SpawnDefaultController _returnvalue_3)
            (Class|CombatInterface|IncrementMinionCount(Message) (Variables|Default|GetOwningActor) 1)
            (Math|Integer|IncrementInt (Variables|Default|GetSpawnLocationIndex)
              (:%20%20
                (Utilities|FlowControl|Delay 0.2)
                (goto _label)))
            (else
              (Ability|EndAbility))))))
    (:OnCompleted
      (Ability|EndAbility :!label _label_2))
    (:OnInterrupted
      (goto _label_2))
    (:OnCancelled
      (goto _label_2))))