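; Arcane Shards ability: shows a magic circle, then on press commits and spawns shards around the cursor's ground hit.
; A spawned BP_PointCollection supplies one ground point per ability level.
; After the cast montage event, a looping timer fires a GameplayCue at each point and applies radial damage with outward knockback and death impulse.
; MakeAbilityDesc formats level, damage, mana cost and cooldown into the description.
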(event Custom|SpawnShard
  (bind _returnvalue (Ability|GetAvatarActorfromActorInfo))
  (if (< (Variables|Default|GetCount) (Variables|Default|GetNumPoints))
    ;[0.09873 1 0.8742] 触发cue
    (Variables|Default|SetRadialOrigin (Transformation|GetWorldLocation (Utilities|Array|Get(acopy) (Variables|Default|GetGroundPoints) (Variables|Default|GetCount))))
    (Class|GameplayAbility|ExecuteGameplayCuewithParams "(TagName=\"GameplayCue.ArcaneShards\")" (Ability|GameplayCue|MakeGameplayCueParameters :Location (Variables|Default|GetRadialOrigin)))
    (Math|Integer|IncrementInt (Variables|Default|GetCount)
      (:%20%20
        ;[1 0.5257 0.1137] 范围伤害
        (bind _outoverlappingactors (Class|AuraAbilitySystemLibrary|GetLivePlayersWithinRadius _returnvalue (Utilities|Array|MakeArray _returnvalue) (Variables|Default|GetRadialDamageOuterRadius) (Variables|Default|GetRadialOrigin)))
        (bind _output_get (Variables|Default|SetOverlappingActors _outoverlappingactors))
        (for _array_element _output_get
          (Variables|Default|SetTargetActor _array_element)
          (Class|AuraAbilitySystemLibrary|ApplyDamageEffect (Class|AuraDamageGameplayAbility|MakeDamageEffectParamfromClassDefaults (Variables|Default|GetTargetActor) (Variables|Default|GetRadialOrigin) true (- (Transformation|GetActorLocation (Variables|Default|GetTargetActor)) (Variables|Default|GetRadialOrigin)) true (- (Transformation|GetActorLocation (Variables|Default|GetTargetActor)) (Variables|Default|GetRadialOrigin)) true 45.0)))))
    (else
      (Utilities|FlowControl|Delay 0.2)
      (Actor|DestroyActor (Variables|Default|GetPointCollection))
      (Utilities|Time|ClearandInvalidateTimerbyHandle (Variables|Default|GetSpawnShardTimeHandle))
      (Ability|EndAbility))))

(event Ability|EventActivateAbility
  (Utilities|FlowControl|Sequence
    (:then_0
      (Class|PlayerInterface|ShowMagicCircle(Message) (Ability|GetAvatarActorfromActorInfo) 0)
      (Variables|Default|SetNumPoints (Ability|GetAbilityLevel)))
    (:then_1
      (Ability|Tasks|WaitInputPress false
        (:OnPress
          (bind _returnvalue (Ability|CommitAbility))
          (if _returnvalue
            (bind _datahandle (|TargetDataUnderMouse)
              (:ValidData
                (Variables|Default|SetMouseHitLocation (.ImpactPoint (Collision|BreakHitResult (Ability|TargetData|GetHitResultfromTargetData _datahandle))))
                ;[0.4609 1 0.4952] 创建一个空模型actor 作用是找到当前鼠标附件的各个点位 用来防止ArcaneShards的NiagaraSystem
                (bind _returnvalue_2 (Game|SpawnActorfromClass "/Game/Blueprints/AbilitySystem/Aura/Abilities/Arcane/ArcaneShards/BP_PointCollection.BP_PointCollection_C" (Math|Transform|MakeTransform (Variables|Default|GetMouseHitLocation) "0, 0, 0" "1.000000,1.000000,1.000000") "AlwaysSpawn" "MultiplyWithRoot" 0 0))
                (Variables|Default|SetPointCollection _returnvalue_2)
                (Variables|Default|SetGroundPoints (Class|PointCollection|GetGroundPoint (Variables|Default|GetPointCollection) (Variables|Default|GetMouseHitLocation) (Variables|Default|GetNumPoints) 0.0))
                (Variables|Default|SetCount 0)
                (Class|CombatInterface|UpdateFacingTarget(Message) (Ability|GetAvatarActorfromActorInfo) (Variables|Default|GetMouseHitLocation))
                (|PlayMontageandWaitProxy "None" "/Game/Assets/Characters/Aura/Animations/Abilities/AM_Cast_ArcaneShards.AM_Cast_ArcaneShards" 1.0 "None" false 1.0 0.0
                  (:then
                    (Ability|Tasks|WaitGameplayEvent "(TagName=\"Event.Montage.ArcaneShards\")" 0 true
                      (:EventReceived
                        (bind _returnvalue_3 (Utilities|Time|SetTimerbyEvent (delegate Custom|SpawnShard) (Variables|Default|GetShardSpawnDeltaTime) true -0.2))
                        (Variables|Default|SetSpawnShardTimeHandle _returnvalue_3)
                        (Class|PlayerInterface|HideMagicCircle(Message) (Ability|GetAvatarActorfromActorInfo))))))))
            (else
              (Ability|EndAbility))))))))

(event Ability|EventOnEndAbility
  (params (bWasCancelled :type Boolean)))

(fn MakeAbilityDesc
  (params (InFormat :type Text%20%28by%20ref%29) (Level :type Integer))
  (LocalVariables|SetInputLevel Level)
  (return (Utilities|Text|FormatText InFormat (LocalVariables|GetInputLevel) (Class|AuraDamageGameplayAbility|GetDamagebyLevel (Math|Conversions|ToFloat(Integer) (LocalVariables|GetinputLevel))) (* (Class|AuraGameplayAbility|GetManaCost (Math|Conversions|ToFloat(Integer) (LocalVariables|GetinputLevel))) -1.0) (Class|AuraGameplayAbility|GetCooldown (Math|Conversions|ToFloat(Integer) (LocalVariables|GetinputLevel))))))