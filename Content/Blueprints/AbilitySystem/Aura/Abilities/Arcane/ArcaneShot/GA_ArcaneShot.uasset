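; Gameplay ability for Arcane Shot that spawns arcane stones and then launches them.
; On activation it commits, takes target data under the mouse and turns the avatar to face that location through the CombatInterface.
; It plays the cast montage, whose gameplay events trigger spawning and launching the stones.
; The ability ends when the montage completes, blends out, or is interrupted or cancelled.
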(event Ability|EventActivateAbility
  (Ability|CommitAbility)
  (bind _datahandle (|TargetDataUnderMouse)
    (:ValidData
      (Variables|Default|SetMouseHitActor (.HitActor (Collision|BreakHitResult (Ability|TargetData|GetHitResultfromTargetData _datahandle))))
      (bind _output_get (Variables|Default|SetTargetLocation (.Location (Collision|BreakHitResult (Ability|TargetData|GetHitResultfromTargetData _datahandle)))))
      (bind _ascombat_interface (Utilities|Casting|CastToCombatInterface (Ability|GetAvatarActorfromActorInfo)))
      (Class|CombatInterface|UpdateFacingTarget _ascombat_interface _output_get)
      (|PlayMontageandWaitProxy "None" "/Game/Assets/Characters/Aura/Animations/Abilities/AM_Cast_ArcaneShot.AM_Cast_ArcaneShot" 1.0 "None" false 1.0 0.0
        (:then
          ;[0.22 1 0.7591] 生成奥术飞弹
          (Ability|Tasks|WaitGameplayEvent "(TagName=\"Event.Montage.ArcaneStoneSpawn\")" 0 true
            (:then
              ;[0.1629 1 0.2536] 释放奥术飞弹
              (Ability|Tasks|WaitGameplayEvent "(TagName=\"Event.Montage.ArcaneStoneShot\")" 0 true
                (:EventReceived
                  (Class|AuraStoneShot|LaunchAllStones))))
            (:EventReceived
              (Class|AuraStoneShot|SpawnStones))))
        (:OnCompleted
          (Ability|EndAbility :!label _label))
        (:OnBlendOut
          (goto _label))
        (:OnInterrupted
          (goto _label))
        (:OnCancelled
          (goto _label))))))

(event Ability|EventOnEndAbility
  (params (bWasCancelled :type Boolean)))