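; Passive startup ability that listens for Attributes gameplay events and turns them into gameplay effects on its owner.
; Exact IncomingExp events apply the experience effect, and Primary attribute events apply the base-attribute effect.
; Each event's tag and magnitude feed the effect spec as SetByCaller values.
; For primary attributes, ClearSpecMagnitude first zeroes every base-attribute tag on a spec made from that effect class.
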(event Ability|EventActivateAbility
  (bind _eventbasedeffectclass_baseattr (Variables|Default|GetEventBasedEffectClass_BaseAttr))
  (bind _returnvalue (Ability|MakeOutgoingGameplayEffectSpec _eventbasedeffectclass_baseattr))
  (bind _payload (Ability|Tasks|WaitGameplayEvent "(TagName=\"Attributes\")" 0 false false)
    (:EventReceived
      (Variables|Default|SetEvent%20Magnitude (.EventMagnitude (Utilities|Struct|BreakGameplayEventData _payload)))
      (bind _output_get (Variables|Default|SetReciveEventTag (.EventTag (Utilities|Struct|BreakGameplayEventData _payload))))
      (if (GameplayTags|MatchesTag _output_get "(TagName=\"Attributes.Meta.IncomingExp\")" true)
        (bind _returnvalue_2 (Ability|GameplayEffect|AssignTagSetbyCallerMagnitude (Ability|MakeOutgoingGameplayEffectSpec (Variables|Default|GetEventBasedEffectClass_Exp)) (Variables|Default|GetReciveEventTag) (Variables|Default|GetEvent%20Magnitude)))
        (GameplayEffects|ApplyGameplayEffectSpecToSelf (Ability|GetAbilitySystemComponentfromActorInfo) _returnvalue_2)
        (elif (GameplayTags|MatchesTag (Variables|Default|GetReciveEventTag) "(TagName=\"Attributes.Primary\")")
          (CallFunction|ClearSpecMagnitude _returnvalue)
          (bind _returnvalue_3 (Ability|GameplayEffect|AssignTagSetbyCallerMagnitude _returnvalue (Variables|Default|GetReciveEventTag) (Variables|Default|GetEvent%20Magnitude)))
          (GameplayEffects|ApplyGameplayEffectSpecToSelf (Ability|GetAbilitySystemComponentfromActorInfo) _returnvalue_3))))))

(fn ClearSpecMagnitude
  (params (SpecHandle :type Gameplay%20Effect%20Spec%20Handle%20Structure))
  (for _array_element (GameplayTags|BreakGameplayTagContainer (Variables|Default|GetBaseAttrTags))
    (Ability|GameplayEffect|AssignTagSetbyCallerMagnitude SpecHandle _array_element 0.0)))