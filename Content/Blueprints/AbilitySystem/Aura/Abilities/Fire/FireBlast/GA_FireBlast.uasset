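; GA_FireBlast is the Fire Blast gameplay ability, which spawns fireballs when activated.
; Activation commits the ability, calls SpawnFireBalls, which is defined outside this graph, and ends immediately.
; MakeAbilityDesc fills a supplied text format with level, damage, negated mana cost and cooldown for that level.
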(event Ability|EventActivateAbility
  (Ability|CommitAbility)
  (Class|AuraFireBlast|SpawnFireBalls)
  (Ability|EndAbility))

(event Ability|EventOnEndAbility
  (params (bWasCancelled :type Boolean)))

(fn MakeAbilityDesc
  (params (InFormat :type Text%20%28by%20ref%29) (Level :type Integer))
  (LocalVariables|SetInputLevel Level)
  (return (Utilities|Text|FormatText InFormat (LocalVariables|GetInputLevel) (Class|AuraDamageGameplayAbility|GetDamagebyLevel (Math|Conversions|ToFloat(Integer) (LocalVariables|GetinputLevel))) (* (Class|AuraGameplayAbility|GetManaCost (Math|Conversions|ToFloat(Integer) (LocalVariables|GetinputLevel))) -1.0) (Class|AuraGameplayAbility|GetCooldown (Math|Conversions|ToFloat(Integer) (LocalVariables|GetinputLevel))))))