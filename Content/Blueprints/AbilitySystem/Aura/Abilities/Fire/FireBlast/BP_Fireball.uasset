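; BP_Fireball is a Fire Blast projectile that flies out, returns toward its return actor and explodes.
; On authority, a timeline lerps it forward by TravelDistance, then a second timeline plays in reverse toward the return actor's position sampled at turnaround.
; Return updates call OnHit; within ExplodeDistance, it applies radial damage with flattened knockback directions to nearby live actors, excluding itself and its owner, then destroys itself.
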(event EventBeginPlay)

(event Collision|EventActorBeginOverlap
  (params (OtherActor :type Actor%20Object%20Reference)))

(event EventTick
  (params (DeltaSeconds :type Float%20%28single-precision%29)))

(event EventStartOutgoingTimeline
  (bind _returnvalue (Class|AuraFireBall|GetReturnActor))
  (Networking|SwitchHasAuthority
    (:Authority
      ;[0.5576 1 0.1271] 计算起点和终点
      (Variables|Default|SetInitialLocation (Transformation|GetActorLocation))
      (Variables|Default|SetApexLocation (+ (Variables|Default|GetInitialLocation) (* (Transformation|GetActorForwardVector) (Variables|Default|GetTravelDistance))))
      ;[1 0.9418 0.09919] 在两点间用timeline插值
      (bind _outgoingtrack (Timeline|OutgoingTimeline PlayFromStart)
        (:Update
          (Transformation|SetActorLocation (Math|Vector|Lerp(Vector) (Variables|Default|GetInitialLocation) (Variables|Default|GetApexLocation) _outgoingtrack) false false))
        (:Finished
          ;[1 0.3849 0.08671] 更新起始点的位置，用相反的timeline插值
          (Utilities|IsValid _returnvalue
            (:Is%20Valid
              (Variables|Default|SetInitialLocation (Transformation|GetActorLocation _returnvalue))
              (bind _outgoingtrack_2 (Timeline|OutGoingTimelineCopy ReverseFromEnd)
                (:Update
                  (Transformation|SetActorLocation (Math|Vector|Lerp(Vector) (Variables|Default|GetInitialLocation) (Variables|Default|GetApexLocation) _outgoingtrack_2) false false)
                  ;[1 0.02194 0.06373] server调用 client会在destroy的时候调用，别问为什么这么写
                  (Class|AuraProjectile|OnHit)
                  (if (<= (Math|Vector|VectorLength (- (Transformation|GetActorLocation) (Variables|Default|GetInitialLocation))) (Variables|Default|GetExplodeDistance))
                    ;[0.09605 0.5294 1] 在返回的最后时刻调用OnHit爆炸 然后对周围的敌人施加RadialDamage
                    (Class|AuraAbilitySystemLibrary|SetIsRadialDamageEffectParams (Variables|Default|GetExplosionDamageParams) true 5e+01 3e+02 (Transformation|GetActorLocation))
                    (Variables|Default|SetPlayersAroundBall (Utilities|Array|MakeArray (Components|GetOwner)))
                    (Utilities|Array|Add (Variables|Default|GetPlayersAroundBall) self)
                    (bind _outoverlappingactors (Class|AuraAbilitySystemLibrary|GetLivePlayersWithinRadius self (Variables|Default|GetPlayersAroundBall) 3e+02 (Transformation|GetActorLocation)))
                    (for _array_element _outoverlappingactors
                      (Class|AuraAbilitySystemLibrary|SetEffectParamsTargetASC (Variables|Default|GetExplosionDamageParams) (Ability|GetAbilitySystemComponent _array_element))
                      (Variables|Default|SetKnockbackDirection (- (Transformation|GetActorLocation _array_element) (Transformation|GetActorLocation)))
                      (Class|AuraAbilitySystemLibrary|SetImpulseDirection (Variables|Default|GetExplosionDamageParams) (Math|Vector|GetForwardVector (Math|Rotator|MakeRotator (.roll (Math|Rotator|MakeRotfromX (Variables|Default|GetKnockbackDirection))) 0.0 (.yaw (Math|Rotator|MakeRotfromX (Variables|Default|GetKnockbackDirection))))) 0.0)
                      (Class|AuraAbilitySystemLibrary|SetKnockbackDirection (Variables|Default|GetExplosionDamageParams) (Math|Vector|GetForwardVector (Math|Rotator|MakeRotator (.roll (Math|Rotator|MakeRotfromX (Variables|Default|GetKnockbackDirection))) 0.0 (.yaw (Math|Rotator|MakeRotfromX (Variables|Default|GetKnockbackDirection))))) 0.0)
                      (Class|AuraAbilitySystemLibrary|ApplyDamageEffect (Variables|Default|GetExplosionDamageParams)))
                    (Actor|DestroyActor)))
                (:Finished
                  (Actor|DestroyActor))))))))))

(fn ConstructionScript)