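; GA_Electrocute is a channeled lightning ability that shocks the first traced target toward the cursor, chaining to level-scaled extra targets.
; A montage event roots the caster, adds ShockLoop gameplay-cue beams and starts a looping timer that commits cost and applies damage.
; Input release (after a minimum hold), failed cost or primary-target death ends it, applying an authority-only final hit with debuff/knockback, then cooldown.
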(event Custom|DamageAndCost
  (bind _returnvalue (Ability|CommitAbilityCost false))
  (if _returnvalue
    (CallFunction|ApplyDamage)
    (else
      (CallFunction|AbilityEnd))))

(event Ability|EventActivateAbility
  (if (Utilities|DoesObjectImplementInterface (Ability|GetAvatarActorfromActorInfo) "/Script/PJ_AURA.CombatInterface")
    ;[1 0.307 0.8549] store mouse data var
    (bind _datahandle (|TargetDataUnderMouse)
      (:ValidData
        (Class|AuraBeamSpell|StoreMouseDataInfo (Ability|TargetData|GetHitResultfromTargetData _datahandle))
        (Class|AuraBeamSpell|StoreOwnerInfo)
        (Utilities|FlowControl|Sequence
          (:then_0
            (Variables|/Script/Engine.PlayerController|SetbShowMouseCursor (Variables|Default|GetOwnerPlayerController) false)
            (Class|CombatInterface|UpdateFacingTarget(Message) (Ability|GetAvatarActorfromActorInfo) (Variables|Default|GetMouseHitLocation))
            (GameplayCue|ExecuteGameplayCue :GameplayCueTag "(TagName=\"GameplayCue.ShockBurst\")")
            (|PlayMontageandWaitProxy "None" (Variables|Default|GetMontage_Electrocute) 1.0 "None" true 1.0 0.0
              (:then
                ;[1 0.7612 0.1685] 这里直接调用的原因是：playmontage的时候动画状态机的控制是被 montage接管的，不会立马进入shockloop阶段。
                ; 而是在montage结束时混合montage的收尾动作与shockkoop的开头动作。
                (Class|CombatInterface|SetinShockLoop(Message) (Ability|GetAvatarActorfromActorInfo) true)
                (Ability|Tasks|WaitGameplayEvent "(TagName=\"Event.Montage.Electrocute\")" 0 true
                  (:EventReceived
                    (Pawn|Components|CharacterMovement|DisableMovement (Variables|/Script/Engine.Character|GetCharacterMovement (Variables|Default|GetOwnerCharacter)))
                    (CallFunction|SpawnElectricBeam)
                    (bind _returnvalue (Utilities|Time|SetTimerbyEvent (delegate Custom|DamageAndCost) (Variables|Default|GetDamageDeltaTime) true))
                    (Variables|Default|SetDamageAndCostTimer _returnvalue)
                    (CallFunction|DamageandCost))))))
          (:then_1
            (bind _timeheld (Ability|Tasks|WaitInputRelease false)
              (:OnRelease
                (bind _output_get (Variables|Default|SetTime%20Held _timeheld))
                (if (< _output_get (Variables|Default|GetMiniSpellTime))
                  (Ability|HasAuthority
                    (:True
                      (Utilities|FlowControl|Delay (- (Variables|Default|GetMiniSpellTime) (Variables|Default|GetTime%20Held)))
                      (CallFunction|AbilityEnd :!label _label))
                    (:False
                      (Variables|/Script/Engine.PlayerController|SetbShowMouseCursor (Variables|Default|GetOwnerPlayerController) true)))
                  (else
                    (goto _label)))))))))
    (else
      (Ability|EndAbility))))

(event EventPrimaryActorDied
  (params (DeadActor :type Actor%20Object%20Reference))
  (CallFunction|AbilityEnd))

(event EventAdditionalActorDied
  (params (DeadActor :type Actor%20Object%20Reference))
  (bind _additionalactorstocueparams (Variables|Default|GetAdditionalActorsToCueParams))
  (bind (_value _returnvalue) (Utilities|Map|Find _additionalactorstocueparams DeadActor))
  (Utilities|IsValid DeadActor
    (:Is%20Valid
      (if _returnvalue
        (GameplayCue|RemoveGameplayCueOnActor(Looping) DeadActor "(TagName=\"GameplayCue.ShockLoop\")" _value)
        (Utilities|Map|Remove (Variables|Default|GetAdditionalActorsToCueParams) DeadActor)
        (Utilities|Array|RemoveItem (Variables|Default|GetAdditional%20Targets) DeadActor)))))

(fn SpawnElectricBeam
  ;[0.1383 1 0.2366] 更新mousehitlocation和hitactor为射线第一个击中的敌人
  (Class|AuraBeamSpell|TraceFirstTarget (Variables|Default|GetMouseHitLocation))
  (bind _returnvalue (Class|CombatInterface|GetWeapon(Message) (Variables|Default|GetOwnerCharacter)))
  (Variables|Default|SetFirstTargetCueParams (Ability|GameplayCue|MakeGameplayCueParameters :Location (Variables|Default|GetMouseHitLocation) :SourceObject (Variables|Default|GetMouseHitActor) :TargetAttachComponent _returnvalue))
  ;[1 0.8582 0.1061] 击中的第一个是否是敌人
  (bind _output_get (Variables|Default|SetFirstTargetPassing (Utilities|DoesObjectImplementInterface (Variables|Default|GetMouseHitActor) "/Script/PJ_AURA.CombatInterface")))
  (if _output_get
    (LocalVariables|SetCueTarget (Variables|Default|GetMouseHitActor))
    (else
      (LocalVariables|SetCueTarget (Variables|Default|GetOwnerCharacter))))
  ;[0.1256 0.5648 1] 第一段闪电
  (GameplayCue|AddGameplayCueOnActor(Looping) (LocalVariables|GetCueTarget) "(TagName=\"GameplayCue.ShockLoop\")" (Variables|Default|GetFirstTargetCueParams))
  (if (Variables|Default|GetFirstTargetPassing)
    (Class|CombatInterface|SetBeingShocked(Message) (LocalVariables|GetCueTarget) true)
    (Variables|Default|SetMaxBroadTarget (Math|Integer|Clamp(Integer) (- (Ability|GetAbilityLevel) 1) 0 (Variables|Default|GetMaxBroadTarget)))
    (bind _outadditionaltargets (Class|AuraBeamSpell|StoreAdditionalTargets (Variables|Default|GetMaxBroadTarget)))
    (bind _output_get_2 (Variables|Default|SetAdditional%20Targets _outadditionaltargets))
    (for _array_element _output_get_2
      (CallFunction|AddShockLoopCuetoAdditionalTarget _array_element)
      (Class|CombatInterface|SetBeingShocked(Message) _array_element true))))

(fn AddShockLoopCuetoAdditionalTarget
  (params (AdditionalTarget :type Actor%20Object%20Reference))
  (LocalVariables|SetTargetActor AdditionalTarget)
  (LocalVariables|SetCueParam (Ability|GameplayCue|MakeGameplayCueParameters :Location (Transformation|GetActorLocation (LocalVariables|GetTargetActor)) :SourceObject (LocalVariables|GetTargetActor) :TargetAttachComponent (Variables|/Script/Engine.Actor|GetRootComponent (Variables|Default|GetMouseHitActor))))
  (Utilities|Map|Add (Variables|Default|GetAdditionalActorsToCueParams) (LocalVariables|GetTargetActor) (LocalVariables|GetCueParam))
  (GameplayCue|AddGameplayCueOnActor(Looping) (LocalVariables|GetTargetActor) "(TagName=\"GameplayCue.ShockLoop\")" (LocalVariables|GetCueParam)))

(fn AbilityEnd
  (bind _mousehitactor (Variables|Default|GetMouseHitActor))
  (Utilities|Time|ClearandInvalidateTimerbyHandle (Variables|Default|GetDamageAndCostTimer))
  (Variables|/Script/Engine.PlayerController|SetbShowMouseCursor (Variables|Default|GetOwnerPlayerController) true)
  (Class|CombatInterface|SetinShockLoop(Message) (Ability|GetAvatarActorfromActorInfo) false)
  (Pawn|Components|CharacterMovement|SetMovementMode (Variables|/Script/Engine.Character|GetCharacterMovement (Variables|Default|GetOwnerCharacter)) "MOVE_Walking" 0)
  (if (Variables|Default|GetFirstTargetPassing)
    (Class|CombatInterface|SetBeingShocked(Message) _mousehitactor false)
    (GameplayCue|RemoveGameplayCueOnActor(Looping) _mousehitactor "(TagName=\"GameplayCue.ShockLoop\")" (Variables|Default|GetFirstTargetCueParams))
    (Ability|HasAuthority
      (:True
        ;[1 0.8034 0.1291] 最后一击的时候用ability的effectParam来打伤害，这一次会计算debuff和击退等等
        (Class|AuraAbilitySystemLibrary|ApplyDamageEffect (Class|AuraDamageGameplayAbility|MakeDamageEffectParamfromClassDefaults (Variables|Default|GetMouseHitActor) "0, 0, 0" false "0, 0, 0" false "0, 0, 0" false 0.0)))
      (:False
        _))
    ;[1 0.1281 0.1281] 从散射的其他actor身上删除systen
    (for _array_element (Variables|Default|GetAdditional%20Targets)
      (if (.ReturnValue (Utilities|Map|Find (Variables|Default|GetAdditionalActorsToCueParams) _array_element))
        (Class|CombatInterface|SetBeingShocked(Message) _array_element false)
        (GameplayCue|RemoveGameplayCueOnActor(Looping) _array_element "(TagName=\"GameplayCue.ShockLoop\")" (.Value (Utilities|Map|Find (Variables|Default|GetAdditionalActorsToCueParams) _array_element)))
        (Ability|HasAuthority
          (:True
            (Class|AuraAbilitySystemLibrary|ApplyDamageEffect (Class|AuraDamageGameplayAbility|MakeDamageEffectParamfromClassDefaults _array_element "0, 0, 0" false "0, 0, 0" false "0, 0, 0" false 0.0))))))
    (else
      (GameplayCue|RemoveGameplayCueOnActor(Looping) (Variables|Default|GetOwnerCharacter) "(TagName=\"GameplayCue.ShockLoop\")" (Variables|Default|GetFirstTargetCueParams))))
  (Ability|CommitAbilityCooldown false)
  (CallFunction|ClearParams)
  (Ability|EndAbility))

(fn ApplyDamage
  (CallFunction|ApplySingleDamage (Variables|Default|GetMouseHitActor))
  (for _array_element (Variables|Default|GetAdditional%20Targets)
    (CallFunction|ApplySingleDamage _array_element)))

(fn ApplySingleDamage
  (params (Actor :type Actor%20Object%20Reference))
  (LocalVariables|SetInActor Actor)
  (Utilities|IsValid (LocalVariables|GetInActor)
    (:Is%20Valid
      (LocalVariables|SetApplingASC (Ability|GetAbilitySystemComponentfromActorInfo))
      (bind _returnvalue (Ability|GameplayEffect|AssignTagSetbyCallerMagnitude (GameplayEffects|MakeOutgoingSpec (LocalVariables|GetApplingASC) (Variables|Default|GetDamageEffectClass) (Math|Conversions|ToFloat(Integer) (Ability|GetAbilityLevel)) (GameplayEffects|MakeEffectContext (LocalVariables|GetApplingASC))) "(TagName=\"Damage.Lighting\")" (Class|AuraDamageGameplayAbility|GetDamagebyLevel (Math|Conversions|ToFloat(Integer) (Ability|GetAbilityLevel)))))
      (Utilities|IsValid (Ability|GetAbilitySystemComponent (LocalVariables|GetInActor))
        (:Is%20Valid
          (GameplayEffects|ApplyGameplayEffectSpecToSelf (Ability|GetAbilitySystemComponent (LocalVariables|GetInActor)) _returnvalue))))))

(fn ClearParams
  (Utilities|Array|Clear (Variables|Default|GetAdditional%20Targets))
  (Utilities|Map|Clear (Variables|Default|GetAdditionalActorsToCueParams))
  (Variables|Default|SetMouseHitActor 0)
  (Variables|Default|SetFirstTargetPassing false)
  (Variables|Default|SetTime%20Held 0.0))

(fn MakeAbilityDesc
  (params (InFormat :type Text%20%28by%20ref%29) (Level :type Integer))
  (LocalVariables|SetInputLevel Level)
  (return (Utilities|Text|FormatText InFormat (LocalVariables|GetInputLevel) (Class|AuraDamageGameplayAbility|GetDamagebyLevel (Math|Conversions|ToFloat(Integer) (LocalVariables|GetInputLevel))) (* (Class|AuraGameplayAbility|GetManaCost (Math|Conversions|ToFloat(Integer) (LocalVariables|GetInputLevel))) -1.0) (Class|AuraGameplayAbility|GetCooldown (Math|Conversions|ToFloat(Integer) (LocalVariables|GetInputLevel))))))