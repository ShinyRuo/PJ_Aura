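; Base pickup effect actor, apparently for potions, that animates its spawn and plays spawn and consume sounds.
; On BeginPlay, a timeline drives scale and height scaled by SpawnApex, with a one-shot ground sound triggered by a height threshold.
; When the timeline finishes, it starts rotation and sinusoidal movement.
; Tick applies CalculatedLocation and CalculatedRotation to the actor, and destruction plays the consume sound.
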(event EventBeginPlay
  (bind _calculatedlocation (Variables|Default|GetCalculatedLocation))
  (Audio|PlaySoundatLocation "/Game/Assets/Sounds/Potions/Spawn/sfx_Potion_Spawn.sfx_Potion_Spawn" (Transformation|GetActorLocation) "0, 0, 0" 1.0 1.0 0.0 0 0 0 0)
  (bind (_direction _elevation _scale) (Timeline|PickUpElevationTimeline Play)
    (:Update
      (Transformation|SetActorLocation (Math|Vector|MakeVector (.x _calculatedlocation) (.y _calculatedlocation) (+ (.z _calculatedlocation) (* _elevation (Variables|Default|GetSpawnApex)))) false false)
      (Transformation|SetActorScale3D (Math|Conversions|ToVector(Float) _scale))
      (if (> (+ (.z _calculatedlocation) (* _elevation (Variables|Default|GetSpawnApex))) 0.3)
        (Utilities|FlowControl|DoOnce false
          (:Completed
            (Audio|PlaySoundatLocation (Variables|Default|GetGroundSoundBase) (Transformation|GetActorLocation) "0, 0, 0" 1.0 1.0 0.0 0 0 0 0)))))
    (:Finished
      (Class|AuraEffectActor|StartRotation)
      (Class|AuraEffectActor|StartSinusoidalMovement))))

(event EventDestroyed
  (Audio|PlaySoundatLocation "/Game/Assets/Sounds/Potions/Consume/sfx_Potion_Consume.sfx_Potion_Consume" (Transformation|GetActorLocation) "0, 0, 0" 1.0 1.0 0.0 0 0 0 0))

(event EventTick
  (params (DeltaSeconds :type Float%20%28single-precision%29))
  (Transformation|SetActorLocation (Variables|Default|GetCalculatedLocation) false false)
  (Transformation|SetActorRotation (Variables|Default|GetCalculatedRotation)))

(fn ConstructionScript)